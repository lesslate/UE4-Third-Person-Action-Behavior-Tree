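; BP_RaidPlayerController is the raid player controller that owns the in-game HUD and pause menu UI.
; On BeginPlay it creates the HUD and menu widgets and adds them hidden, along with the settings widget held by BP_GameInstance.
; The VisibleHud event reveals the HUD on demand.
; MenuKey shows the pause menu, switches to UI-only input, pauses the game and shows the cursor.
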(event `self.ReceiveBeginPlay`
  (bind _returnvalue (`|CreateWidget` "/Game/UI/BP_HUDWidget.BP_HUDWidget_C"))
  (bind _output_get (set `self.HUD` _returnvalue))
  (`UserWidget.AddToViewport` _output_get 0)
  (`Widget.SetVisibility` _output_get "Hidden")
  (bind _returnvalue_2 (`|CreateWidget` "/Game/UI/BP_Menu.BP_Menu_C"))
  (bind _output_get_2 (set `self.PauseUI` _returnvalue_2))
  (`UserWidget.AddToViewport` _output_get_2 0)
  (`Widget.SetVisibility` _output_get_2 "Hidden")
  (bind _asbp_game_instance (cast `/Game/GameMode/BP_GameInstance` (`GameplayStatics.GetGameInstance`)))
  (bind _settingwidget (`/Game/GameMode/BP_GameInstance.SettingWidget` _asbp_game_instance))
  (`UserWidget.AddToViewport` _settingwidget 0)
  (`Widget.SetVisibility` _settingwidget "Hidden"))

(event `Key|M`
  (params (Key :type "Key Structure")))

(event `InputAction|MenuKey`
  (params (Key :type "Key Structure"))
  (bind _pauseui (`self.PauseUI`))
  (:`Pressed`
    (`Widget.SetVisibility` _pauseui "Visible")
    (`WidgetBlueprintLibrary.SetInputMode_UIOnlyEx` self _pauseui)
    (`GameplayStatics.SetGamePaused` true)
    (set `self.bShowMouseCursor` true)))

(event `VisibleHud`
  (`Widget.SetVisibility` (`self.HUD`) "Visible"))

(fn `UserConstructionScript`)