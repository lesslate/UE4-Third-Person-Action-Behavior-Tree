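; Player controller for the title screen that sets the camera and builds the menu UI.
; On BeginPlay, if an actor tagged MainCamera exists, it becomes the view target, then the main menu and a hidden boss-select widget are added to the viewport.
; It also switches to UI-only input with a visible cursor and adds the GameInstance's settings widget hidden, which the SettingVisible event later reveals.
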(event `self.ReceiveBeginPlay`
  (bind _outactors (`GameplayStatics.GetAllActorsWithTag` "MainCamera"))
  (if (> (`KismetArrayLibrary.Array_Length` _outactors) 0)
    (bind _ascamera_actor (cast `CameraActor` (`|GetArrayItem` _outactors)))
    (`self.SetViewTargetWithBlend` _ascamera_actor)
    (bind _returnvalue (`|CreateWidget` "/Game/GameMode/Title/BP_MainUI.BP_MainUI_C" self))
    (bind _output_get (set `self.TitleWidget` _returnvalue))
    (`UserWidget.AddToViewport` _output_get 0)
    (bind _returnvalue_2 (`|CreateWidget` "/Game/GameMode/Title/BP_SelectBoss.BP_SelectBoss_C" self))
    (bind _output_get_2 (set `self.SelectBoss` _returnvalue_2))
    (`UserWidget.AddToViewport` _output_get_2 0)
    (`Widget.SetVisibility` _output_get_2 "Hidden")
    (`WidgetBlueprintLibrary.SetInputMode_UIOnlyEx` self _output_get)
    (set `self.bShowMouseCursor` true)
    (bind _asbp_game_instance (cast `/Game/GameMode/BP_GameInstance` (`GameplayStatics.GetGameInstance`)))
    (bind _settingwidget (`RaidGameInstance.SettingWidget` _asbp_game_instance))
    (`UserWidget.AddToViewport` _settingwidget 0)
    (`Widget.SetVisibility` _settingwidget "Hidden")))

(event `SettingVisible`
  (`Widget.SetVisibility` (`RaidGameInstance.SettingWidget` (stale `self.ReceiveBeginPlay` _asbp_game_instance)) "Visible"))

(fn `UserConstructionScript`)